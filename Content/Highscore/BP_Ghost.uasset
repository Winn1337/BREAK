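; BP_Ghost is a highscore ghost actor that replays a timestamped path of positions.
; On BeginPlay it finds the GameManager and disables its tick if the Positions array is empty.
; Each tick it advances an index through Positions against the GameManager's GameTimer, then snaps to that entry without sweep or interpolation.
; The index only moves forward and stops at the last entry, and only location is replayed.
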(event `self.ReceiveBeginPlay`
  (bind _returnvalue (`GameplayStatics.GetActorOfClass` "/Game/GameManager/GameManager.GameManager_C"))
  (set `self.Game Manager` _returnvalue)
  (if (< (`KismetArrayLibrary.Array_Length` (`self.Positions`)) 1)
    (`self.SetActorTickEnabled` false)))

(event `self.ReceiveTick`
  (params (DeltaSeconds :type "Float (single-precision)"))
  (bind _positions (`self.Positions`))
  (bind (_timestamp _position) (break `/Game/Highscore/S_GhostPosition` (`|GetArrayItem` _positions (`self.CurrentPos`))))
  (while (and (< (`self.CurrentPos`) (- (`KismetArrayLibrary.Array_Length` _positions) 1)) (> (`/Game/GameManager/GameManager.GameTimer` (`self.Game Manager`)) _timestamp))
    (`/Engine/EditorBlueprintResources/StandardMacros.IncrementInt` (`self.CurrentPos`)))
  (`self.K2_SetActorLocation` _position))

(fn `UserConstructionScript`)