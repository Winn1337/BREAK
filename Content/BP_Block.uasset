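; BP_Block is a breakable Geometry Collection block that counts toward the level's win condition when hit.
; Its first Hit increments the GameManager's hit-block count, triggers the win check, enables gravity on the geometry collections and prints debug counts.
; Once hit, Tick runs down a despawn timer, then a Timeline rescales the GeometryCollection and destroys the actor when the scale nears zero.
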(event `self.ReceiveTick`
  (params (DeltaSeconds :type "Float (single-precision)"))
  (if (`self.hit`)
    (bind _output_get (set `self.DespawnTimer` (- (`self.DespawnTimer`) DeltaSeconds)))
    (if (<= _output_get 0.0)
      (bind (_direction _newtrack_0) (`Timeline|Timeline` :`NewTime` 2.0)
        (:`Update`
          _)
        (:`Finished`
          _))
      (bind _output_get_2 (set `self.Scale` (`KismetMathLibrary.MakeVector` _newtrack_0 _newtrack_0 _newtrack_0)))
      (`SceneComponent.SetWorldScale3D` (`self.GeometryCollection`) _output_get_2)
      (if (`KismetMathLibrary.Vector_IsNearlyZero` _output_get_2 0.01)
        (`self.K2_DestroyActor`)))))

(event `self.ReceiveHit`
  (params (MyComp :type "PrimitiveComponent Object Reference") (Other :type "Actor Object Reference") (OtherComp :type "PrimitiveComponent Object Reference") (bSelfMoved :type Boolean) (HitLocation :type "Vector Structure") (HitNormal :type "Vector Structure") (NormalImpulse :type "Vector Structure") (Hit :type "HitResult Structure (by ref)"))
  (bind _gamemanager (`self.gameManager`))
  (if (not (`self.hit`))
    (bind _asgame_manager (cast `/Game/GameManager/GameManager` (`self.gameManager`)))
    (set `/Game/GameManager/GameManager.nrOfHitBlocks` (+ (`/Game/GameManager/GameManager.nrOfHitBlocks` _asgame_manager) 1) _asgame_manager)
    (set `self.hit` true)
    (bind _asgame_manager_2 (cast `/Game/GameManager/GameManager` _gamemanager)
      (:`then`
        (`/Game/GameManager/GameManager.CheckWinCon` _asgame_manager_2))
      (:`CastFailed`
        (`KismetSystemLibrary.PrintString` "Couldnt Find GameManager")))
    (`PrimitiveComponent.SetEnableGravity` (`self.GC_BreakableSurface2`) true)
    (`PrimitiveComponent.SetEnableGravity` (`self.GeometryCollection`) true)
    (bind _asgame_manager_3 (cast `/Game/GameManager/GameManager` _gamemanager))
    (`KismetSystemLibrary.PrintString` (`KismetStringLibrary.Conv_IntToString` (`/Game/GameManager/GameManager.nrOfBlocks` _asgame_manager_3)))
    (`KismetSystemLibrary.PrintString` (`KismetStringLibrary.Conv_IntToString` (`/Game/GameManager/GameManager.nrOfHitBlocks` _asgame_manager_3)))))

(fn `UserConstructionScript`)